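; Goal spawner actor for an experiment that keeps a randomly placed sphere goal within a Border area and tracks how many are removed over time.
; The construction script stretches a plane to preview the area, and BeginPlay resets root scale before spawning the first goal.
; DestroyComponent removes a goal, logs a running count against elapsed time in the Statistic map, and spawns another.
; Once time passes TimeBorder, Tick prints the statistics once.
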(event `self.ReceiveBeginPlay`
  (`SceneComponent.SetWorldScale3D` (`self.DefaultSceneRoot`) (1.0 1.0 1.0))
  (`self.SpawnNewGoal`))

(event `self.ReceiveTick`
  (params (DeltaSeconds :type "Float (single-precision)"))
  (set `self.Time` (+ (`self.Time`) DeltaSeconds))
  (if (> (`self.Time`) (`self.TimeBorder`))
    (`/Engine/EditorBlueprintResources/StandardMacros.DoOnce` false
      (:`Completed`
        (`self.PrintLog` (`self.Statistic`))))))

(fn `DestroyComponent`
  (params (ActorComponent :type "ActorComponent Object Reference"))
  (`/Engine/EditorBlueprintResources/StandardMacros.IsValid` ActorComponent
    (:`Is Valid`
      (`ActorComponent.K2_DestroyComponent` ActorComponent)
      (bind _values (`BlueprintMapLibrary.Map_Values` (`self.Statistic`)))
      (bind _result (`/Engine/EditorBlueprintResources/StandardMacros.IncrementInt` (`|GetArrayItem` _values (`KismetArrayLibrary.Array_LastIndex` _values)))
        (:`  `
          (`BlueprintMapLibrary.Map_Add` (`self.Statistic`) (`self.Time`) _result)
          (`self.SpawnNewGoal`))))))

(fn `UserConstructionScript`
  (bind (_returnvalue_x _returnvalue_y) (`KismetMathLibrary.BreakVector2D` (/ (`self.Border`) 100.0)))
  (`SceneComponent.K2_SetRelativeLocation` (`self.Plane`) (`KismetMathLibrary.MakeVector` (/ (* 1.0 100.0) 2.0) (/ (* 1.0 100.0) 2.0)) false false)
  (`SceneComponent.SetWorldScale3D` (`self.DefaultSceneRoot`) (`KismetMathLibrary.MakeVector` _returnvalue_x _returnvalue_y 1.0)))