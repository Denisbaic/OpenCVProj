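; Actor that runs the webcam calibration UI flow, showing a welcome screen and then the calibration HUD.
; BeginPlay creates the WBP_Wellcome widget, stores it and adds it to the viewport.
; StartCalibrate removes that widget and spawns a BP_WebcamReader with gesture-change reactions disabled.
; It then creates WBP_CalibrateHUD with the delay and calibration timers plus the reader instance, and displays it.
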(event `self.ReceiveBeginPlay`
  (bind _returnvalue (`|CreateWidget` "/Game/Blueprints/WBP_Wellcome.WBP_Wellcome_C"))
  (bind _output_get (set `self.NewVar_0` _returnvalue))
  (`UserWidget.AddToViewport` _output_get 0))

(event `Start Calibrate`
  (params (TimerDelay :type "Float (double-precision)") (TimerToCalibrate :type "Float (double-precision)"))
  (`Widget.RemoveFromParent` (`self.NewVar_0`))
  (bind _returnvalue (`|SpawnActorFromClass` "/Game/Blueprints/BP_WebcamReader.BP_WebcamReader_C" (`KismetMathLibrary.MakeTransform` (0.0 0.0 0.0) (`KismetMathLibrary.MakeRotator` 0.0)) "Undefined" "OverrideRootScale" null null))
  (set `WebcamReader.IsNeedToReactOnGestureChanges` false _returnvalue)
  (bind _returnvalue_2 (`|CreateWidget` "/Game/Blueprints/WBP_CalibrateHUD.WBP_CalibrateHUD_C" null TimerDelay TimerToCalibrate _returnvalue))
  (`UserWidget.AddToViewport` _returnvalue_2 0)
  (`Widget.RemoveFromParent` (`self.NewVar_0`)))

(fn `UserConstructionScript`)