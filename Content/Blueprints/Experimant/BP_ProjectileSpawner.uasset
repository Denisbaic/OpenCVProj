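; BP_ProjectileSpawner is an actor that repeatedly spawns projectiles of a configurable class at its own transform.
; BeginPlay seeds a countdown with a random delay between minimum and maximum spawn times.
; Tick decrements the countdown by frame time, then re-rolls it and spawns a projectile when it drops below zero, giving irregular firing intervals without timers.
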(event `self.ReceiveBeginPlay`
  (set `self.CurrentTimeDelay` (`KismetMathLibrary.RandomFloatInRange` (`self.MinSpawnTime`) (`self.MaxSpawnTime`))))

(event `self.ReceiveTick`
  (params (DeltaSeconds :type "Float (single-precision)"))
  (bind _output_get (set `self.CurrentTimeDelay` (- (`self.CurrentTimeDelay`) DeltaSeconds)))
  (if (< _output_get 0.0)
    (set `self.CurrentTimeDelay` (`KismetMathLibrary.RandomFloatInRange` (`self.MinSpawnTime`) (`self.MaxSpawnTime`)))
    (`|SpawnActorFromClass` (`self.ProjectileClass`) (`self.GetTransform`) "Undefined" "OverrideRootScale" null null)))

(fn `UserConstructionScript`)