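; PC, likely a player controller, drives a frame-by-frame data set and a test mode from input.
; BeginPlay loads the "Data" set, and two actions call NextFrame with opposite flags to step through frames.
; ChangeTestMode enables test mode and tells the first WebcamReader found in the level to change its frame size.
; Axis inputs are empty and the click action only prints a debug string.
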(event `self.ReceiveBeginPlay`
  (`FLD_BPL.LoadDataSet` "Data"))

(event `InputAxis|HelloMouseWheel`
  (params (AxisValue :type "Float (single-precision)")))

(event `InputAxis|TurnX`
  (params (AxisValue :type "Float (single-precision)")))

(event `InputAxis|TurnY`
  (params (AxisValue :type "Float (single-precision)")))

(event `InputAction|helloClick`
  (params (Key :type "Key Structure"))
  (:`Pressed`
    (`KismetSystemLibrary.PrintString` "Hello" true true (struct :`R` 0.169559 :`G` 1.0 :`A` 1.0))))

(event `InputAction|ChangeTestMode`
  (params (Key :type "Key Structure"))
  (:`Pressed`
    (`FLD_BPL.SetTestMode` true)
    (bind _outactors (`GameplayStatics.GetAllActorsOfClass` "/Script/OpenCVProj.WebcamReader"))
    (`WebcamReader.ChangeFrameSize` (`|GetArrayItem` _outactors))))

(event `InputAction|NextFrame`
  (params (Key :type "Key Structure"))
  (:`Pressed`
    (`FLD_BPL.NextFrame` false)))

(event `InputAction|OppositeFrame`
  (params (Key :type "Key Structure"))
  (:`Pressed`
    (`FLD_BPL.NextFrame` true)))

(fn `UserConstructionScript`)