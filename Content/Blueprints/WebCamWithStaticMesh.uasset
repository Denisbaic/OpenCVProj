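; Webcam actor Blueprint that shows the live video feed on a plane mesh and reports a face-tracking eye state.
; BeginPlay creates a dynamic material instance for the plane, and each new video frame writes VideoTexture into its Texture parameter.
; Tick calls the parent and prints IsLeftEyeOpen on screen as debug output.
; Unconnected IsEyeOpen checks with an EAR threshold remain in the graph and never run.
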(event `self.ReceiveBeginPlay`
  (bind _returnvalue (`PrimitiveComponent.CreateDynamicMaterialInstance` (`self.Plane`) 0 "/Game/Material.Material" "Texture"))
  (bind _output_get (set `self.NewVar_0` _returnvalue))
  (`PrimitiveComponent.SetMaterial` (`self.Plane`) 0 _output_get))

(event `self.OnNextVideoFrame`
  (`MaterialInstanceDynamic.SetTextureParameterValue` (`self.NewVar_0`) "Texture" (`self.VideoTexture`)))

(event `self.ReceiveTick`
  (params (DeltaSeconds :type "Float (single-precision)"))
  (`parent.ReceiveTick` DeltaSeconds)
  (`KismetSystemLibrary.PrintString` (`KismetStringLibrary.Conv_BoolToString` (`self.IsLeftEyeOpen`)) true true (struct :`G` 1.0 :`B` 0.016063 :`A` 1.0) DeltaSeconds))

(fn `UserConstructionScript`)