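; Webcam reader Blueprint that turns counted blinks into left or right mouse-style clicks and displays the video feed.
; Each Click event increments BlinkingCount; when click mode turns off, one blink calls LeftClick, two call RightClick, and the count resets.
; OnNextVideoFrame pushes VideoTexture into the dynamic material's Texture parameter.
; A timer-based click evaluation and some debug nodes remain disconnected.
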(event `self.ReceiveBeginPlay`
  (add `self.OnClickModeChange` (delegate `OnClickModeChange_Event`)))

(event `OnClickModeChange_Event` :!signature `self.OnClickModeChange`
  (params (IsEnable :type Boolean))
  (if (not IsEnable)
    (switch `int` (`self.Blinking Count`)
      (:`Default`
        (`KismetSystemLibrary.PrintString` "somhing went wrong")
        (set `self.Blinking Count` 0 :!label _label))
      (:`0`
        (`KismetSystemLibrary.PrintString` "No click"))
      (:`1`
        (`KismetSystemLibrary.PrintString` "Left click")
        (`VirtualCursorFunctionLibrary.LeftClick`)
        (goto _label))
      (:`2`
        (`KismetSystemLibrary.PrintString` "Right click")
        (`VirtualCursorFunctionLibrary.RightClick`)
        (goto _label)))))

(event `self.ReceiveTick`
  (params (DeltaSeconds :type "Float (single-precision)")))

(event `self.OnNextVideoFrame`
  (bind _dynamicmaterial (`self.DynamicMaterial`)
    (:`then`
      (`MaterialInstanceDynamic.SetTextureParameterValue` (`|ConvertAsset` _dynamicmaterial) "Texture" (`self.VideoTexture`)))
    (:`else`)))

(event `self.Click`
  (`/Engine/EditorBlueprintResources/StandardMacros.IncrementInt` (`self.Blinking Count`)))

(event `CustomEvent_0`
  (switch `int` (`self.Blinking Count`)
    (:`Default`
      (`KismetSystemLibrary.PrintString` "somhing went wrong")
      (set `self.Blinking Count` 0 :!label _label_2))
    (:`0`
      (`KismetSystemLibrary.PrintString` "No click"))
    (:`1`
      (`KismetSystemLibrary.PrintString` "Left click")
      (goto _label_2))
    (:`2`
      (`KismetSystemLibrary.PrintString` "Right click")
      (goto _label_2))))

(fn `UserConstructionScript`)