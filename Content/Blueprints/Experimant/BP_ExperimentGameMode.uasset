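; BP_ExperimentGameMode is the game mode for a shooting experiment that reports spawn and shot statistics to debug output.
; Tick compares Spawned with NeedToShoot and, once they match, prints both statistic maps a single time through a DoOnce.
; PrintLog formats map entries as time and count pairs, but a return inside its loop stops it after the first entry.
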(event `self.ReceiveTick`
  (params (DeltaSeconds :type "Float (single-precision)"))
  (if (== (`self.Spawned`) (`self.NeedToShoot`))
    (`/Engine/EditorBlueprintResources/StandardMacros.DoOnce` false
      (:`Completed`
        (`|ExecutionSequence`
          (:`then_0`
            (`KismetSystemLibrary.PrintString` "spawn statistic")
            (`self.PrintLog` (`self.spawn_statistic`)))
          (:`then_1`
            (`KismetSystemLibrary.PrintString` "shooted statistic")
            (`self.PrintLog` (`self.shooted_statistic`))))))))

(fn `UserConstructionScript`)