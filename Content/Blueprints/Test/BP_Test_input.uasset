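; Test Blueprint for input handling that rotates a Cube component and prints debug text.
; CustomEvent maps a vector's X and Y to absolute roll and pitch, while OnWheelInput adds pitch from an axis value.
; An action mapping and the mouse wheel axis only print "Hello".
; Logic to fetch WebcamInstance from BP_HUD and bind CustomEvent to its OnGetInput is disconnected and never runs.
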(event `self.ReceiveBeginPlay`)

(event `CustomEvent`
  (params (Input :type "Vector2D Structure"))
  (`SceneComponent.K2_SetWorldRotation` (`self.Cube`) (`KismetMathLibrary.MakeRotator` (* Input_X 10.0) (* Input_Y 10.0)) false false))

(event `self.ReceiveTick`
  (params (DeltaSeconds :type "Float (single-precision)")))

(event `OnWheelInput`
  (params (AxisInput :type "Float (double-precision)"))
  (`SceneComponent.K2_AddWorldRotation` (`self.Cube`) (`KismetMathLibrary.MakeRotator` 0.0 (* AxisInput 10.0)) false false))

(event `InputAction|NewActionMapping_0`
  (params (Key :type "Key Structure"))
  (:`Pressed`
    (`KismetSystemLibrary.PrintString` "Hello")))

(event `InputAxisKey|MouseWheelAxis`
  (params (AxisValue :type "Float (single-precision)"))
  (`KismetSystemLibrary.PrintString` "Hello"))

(fn `UserConstructionScript`)