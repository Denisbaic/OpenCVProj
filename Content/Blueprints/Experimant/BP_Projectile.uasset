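; BP_Projectile is an experiment projectile that reports spawn and hit statistics to BP_ExperimentGameMode.
; On BeginPlay it increments the game mode's spawn count and logs it against game time.
; When its sphere hits an actor that has an owner or is not a BP_Projectile, it destroys that actor, logs the shot count, then destroys itself.
; Velocity and activation logic for ProjectileMovement is present but never runs.
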(event `self.ReceiveBeginPlay`
  (bind _asbp_experiment_game_mode (cast `/Game/Blueprints/Experimant/BP_ExperimentGameMode` (`GameplayStatics.GetGameMode`)))
  (bind _result (`/Engine/EditorBlueprintResources/StandardMacros.IncrementInt` (`/Game/Blueprints/Experimant/BP_ExperimentGameMode.Spawned` _asbp_experiment_game_mode))
    (:`  `
      (`BlueprintMapLibrary.Map_Add` (`/Game/Blueprints/Experimant/BP_ExperimentGameMode.spawn_statistic` _asbp_experiment_game_mode) (`GameplayStatics.GetTimeSeconds`) _result))))

(event `self.Sphere.OnComponentHit`
  (params (HitComponent :type "PrimitiveComponent Object Reference") (OtherActor :type "Actor Object Reference") (OtherComp :type "PrimitiveComponent Object Reference") (NormalImpulse :type "Vector Structure") (Hit :type "HitResult Structure (by ref)"))
  (if (or (`KismetSystemLibrary.IsValid` (`self.GetOwner` OtherActor)) (!= (`GameplayStatics.GetObjectClass` OtherActor) "BP_Projectile_C"))
    (`self.K2_DestroyActor` OtherActor)
    (bind _asbp_experiment_game_mode (cast `/Game/Blueprints/Experimant/BP_ExperimentGameMode` (`GameplayStatics.GetGameMode`)))
    (bind _result (`/Engine/EditorBlueprintResources/StandardMacros.IncrementInt` (`/Game/Blueprints/Experimant/BP_ExperimentGameMode.Shooted` _asbp_experiment_game_mode))
      (:`  `
        (`BlueprintMapLibrary.Map_Add` (`/Game/Blueprints/Experimant/BP_ExperimentGameMode.shooted_statistic` _asbp_experiment_game_mode) (`GameplayStatics.GetTimeSeconds`) _result)
        (`self.K2_DestroyActor` self)))))

(fn `UserConstructionScript`)